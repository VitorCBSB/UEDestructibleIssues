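; Destructible building that fractures when actors with a contact damage interface overlap it or when it is hit by an attack.
; On overlap it gets the damage from the other actor and calls its own Hit with Attack, directed away from that actor.
; Hit with Attack applies damage to the destructible component, scaling impulse strength with damage, and reports the damage dealt.
; The fracture event is bound on BeginPlay but only prints a debug message.
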(event Custom|On%20Destruction
  (params (HitPoint :type Vector%20%28by%20ref%29) (HitDirection :type Vector%20%28by%20ref%29))
  (Development|PrintString "On Destruction called!"))

(event Collision|EventActorBeginOverlap
  (params (OtherActor :type Actor%20Object%20Reference))
  (bind _returnvalue (Transformation|GetActorLocation))
  (if (Utilities|DoesObjectImplementInterface OtherActor "/Game/Blueprints/Blueprint/Interfaces/ContactDamageInterface.ContactDamageInterface_C")
    (bind _contact_damage (Class|ContactDamageInterface|GetContactDamage(Message) OtherActor))
    (CallFunction|HitwithAttack _returnvalue _contact_damage OtherActor 0 (Math|Vector|Normalize (- _returnvalue (Transformation|GetActorLocation OtherActor))))))

(event EventBeginPlay
  (EventDispatchers|AssignOnComponentFracture (Variables|Default|GetDestructibleComponent) (delegate Custom|On%20Destruction)))

(fn ConstructionScript)

(fn HitwithAttack
  (params (Impact%20Location :type Vector) (Damage :type Float%20%28single-precision%29) (Attacker :type Actor%20Object%20Reference) (Damaging%20Component :type Actor%20Component%20Object%20Reference) (Impact%20Direction :type Vector))
  (Game|Damage|ApplyDamage (Variables|Default|GetDestructibleComponent) Damage Impact%20Location Impact%20Direction (Math|Float|MapRangeClamped Damage 1.0 3e+01 2e+05 1e+06))
  (return Damage "NewEnumerator0"))